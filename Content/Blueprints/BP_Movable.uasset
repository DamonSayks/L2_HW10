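; BP_Movable is a pawn that wanders endlessly between random points within configured bounds.
; From BeginPlay, OnMoved snaps rotation toward a random point, calls AI Move To with a separately evaluated random point, and repeats on success or failure.
; Tick is empty, leaving an older approach disconnected: forward offset movement, sphere-trace reflection off hit surfaces, and re-aiming when outside the 2D boundary check.
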(event `self.ReceiveBeginPlay`
  (`self.OnMoved` 0.0))

(event `self.ReceiveTick`
  (params (DeltaSeconds :type "Float (single-precision)")))

(event `OnMoved`
  (params (Delta :type "Float (double-precision)"))
  (bind (_returnvalue_x _returnvalue_y) (`KismetMathLibrary.BreakVector` (`self.K2_GetActorLocation`)))
  (bind _returnvalue (`KismetMathLibrary.RandomPointInBoundingBox_Box` (make `Box` (`KismetMathLibrary.MakeVector` (`self.Min X`) (`self.Min Y`)) (`KismetMathLibrary.MakeVector` (`self.Max X`) (`self.Max Y`)))))
  ;[1 1 1] Move object
  ;;[1 1 1] AI Move To
  (`self.K2_SetActorRotation` (`KismetMathLibrary.FindLookAtRotation` (`KismetMathLibrary.MakeVector` _returnvalue_x _returnvalue_y) _returnvalue))
  (`|AIMoveTo` self _returnvalue null
    (:`OnSuccess`
      _)
    (:`OnFail`
      _))
  (`self.OnMoved` 0.0))

(event `onRotate`
  (bind (_returnvalue_x _returnvalue_y) (`KismetMathLibrary.BreakVector` (`self.K2_GetActorLocation`)))
  ;[1 1 1] Rotate object
  (`self.K2_SetActorRotation` (`KismetMathLibrary.FindLookAtRotation` (`KismetMathLibrary.MakeVector` _returnvalue_x _returnvalue_y) (`KismetMathLibrary.RandomPointInBoundingBox_Box` (make `Box` (`KismetMathLibrary.MakeVector` (`self.Min X`) (`self.Min Y`)) (`KismetMathLibrary.MakeVector` (`self.Max X`) (`self.Max Y`)))))))

(event `onTrace`
  (bind _scene (`self.Scene`))
  (bind _returnvalue (`SceneComponent.K2_GetComponentLocation` _scene))
  ;[1 1 1] Trace
  (bind (_outhit _returnvalue_2) (`KismetSystemLibrary.SphereTraceSingle` :`Start` _returnvalue :`End` (+ _returnvalue (* (`SceneComponent.GetForwardVector` _scene) (`self.SearchDistance`))) :`TraceChannel` "TraceTypeQuery1" :`DrawDebugType` "ForOneFrame"))
  (if _returnvalue_2
    (`self.K2_SetActorRotation` (`KismetMathLibrary.MakeRotFromX` (`KismetMathLibrary.GetReflectionVector` (`self.GetActorForwardVector`) (`.Normal` (`GameplayStatics.BreakHitResult` _outhit)))))))

(fn `Is Actor in Boundaries 2D`
  (params (`Min X` :type "Float (double-precision)") (`Max X` :type "Float (double-precision)") (`Min Y` :type "Float (double-precision)") (`Max Y` :type "Float (double-precision)"))
  (returns (ReturnValue :type Boolean))
  (bind (_returnvalue_x _returnvalue_y) (`KismetMathLibrary.BreakVector` (`self.K2_GetActorLocation`)))
  (return (and (`KismetMathLibrary.InRange_FloatFloat` _returnvalue_x `Min X` `Max X`) (`KismetMathLibrary.InRange_FloatFloat` _returnvalue_y `Min Y` `Max Y`))))

(fn `UserConstructionScript`)